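; AI controller for the large elf enemy that makes it chase a target pawn.
; On possess it caches the controlled elf, and a SetTargetPlayer event supplies the pawn to follow.
; Each tick it feeds movement input toward the target at half scale along the look-at direction, steering directly without navmesh pathfinding.
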(event Custom|SetTargetPlayer
  (params (TargetPawn :type Pawn%20Object%20Reference))
  (Variables|Default|SetTargetPawn TargetPawn))

(event EventBeginPlay
  (|CallParentFunction) ; This node is disabled and will not be called.\nDrag off pins to build functionality.
)

(event EventTick
  (params (DeltaSeconds :type Float%20%28single-precision%29))
  (|CallParentFunction DeltaSeconds)
  (Variables|Default|GetOwningElf
    (:then
      (Variables|Default|GetTargetPawn
        (:then
          (Default|MoveTowards (Variables|Default|GetOwningElf) (Math|Vector|GetForwardVector (Math|Rotator|FindLookatRotation (Transformation|GetActorLocation (Variables|Default|GetOwningElf)) (Transformation|GetActorLocation (Variables|Default|GetTargetPawn)))) 0.5))
        (:else)))
    (:else)))

(event EventPossess
  (params (PossessedPawn :type Pawn%20Object%20Reference))
  (bind _asbp_enemy_elf_large (Utilities|Casting|CastToBP_Enemy_Elf_Large PossessedPawn))
  (Variables|Default|SetOwningElf _asbp_enemy_elf_large))

(fn ConstructionScript
  (|CallParentFunction))