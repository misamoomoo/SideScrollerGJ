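; Player character Blueprint for a side-scroller, using Paper2D flipbook sprites and Enhanced Input.
; BeginPlay adds the side-scroller mapping context; move input drives movement along world X, and sprint input toggles max walk speed.
; Each tick picks the idle, walk or run flipbook from velocity magnitude against a hardcoded threshold.
; Tick also flips control rotation yaw to face the horizontal direction of travel.
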(event Input|EnhancedActionEvents|EnhancedInputActionIA_Move
  (params (ActionValue :type Float%20%28double-precision%29) (ElapsedSeconds :type Float%20%28double-precision%29) (TriggeredSeconds :type Float%20%28double-precision%29) (InputAction :type Input%20Action%20Object%20Reference :default "/Game/Input/IA_Move.IA_Move"))
  (Pawn|Input|AddMovementInput "1.000000,0.000000,0.000000" ActionValue false))

(event Input|EnhancedActionEvents|EnhancedInputActionIA_Sprint
  (params (ActionValue :type Boolean) (ElapsedSeconds :type Float%20%28double-precision%29) (TriggeredSeconds :type Float%20%28double-precision%29) (InputAction :type Input%20Action%20Object%20Reference :default "/Game/Input/IA_Sprint.IA_Sprint"))
  (bind _charactermovement (Variables|Character|GetCharacterMovement))
  (:Started
    (Variables|/Script/Engine.CharacterMovementComponent|SetMaxWalkSpeed _charactermovement (Variables|Default|GetSprintSpeed)))
  (:Completed
    (Variables|/Script/Engine.CharacterMovementComponent|SetMaxWalkSpeed _charactermovement (Variables|Default|GetWalkSpeed))))

(event EventBeginPlay
  (bind _asplayer_controller (Utilities|Casting|CastToPlayerController (Pawn|GetController)))
  (Input|AddMappingContext (PlayerController|LocalPlayerSubsystems|GetEnhancedInputLocalPlayerSubsystem _asplayer_controller) "/Game/Input/IMC_SideScroller.IMC_SideScroller" 0 "(bIgnoreAllPressedKeysUntilRelease=True,bForceImmediately=False,bNotifyUserSettings=False)"))

(event EventTick
  (params (DeltaSeconds :type Float%20%28single-precision%29))
  (CallFunction|UpdateAnimation)
  (CallFunction|UpdateRotation))

(fn ConstructionScript)

(fn UpdateAnimation
  (if (> (Math|Float|Absolute(Float) (Math|Vector|VectorLength (Transformation|GetVelocity))) 0.0)
    (if (> (Math|Float|Absolute(Float) (Math|Vector|VectorLength (Transformation|GetVelocity))) 6e+02)
      (Sprite|SetFlipbook (Variables|Default|GetSprite) "/Game/Animations/Character/Run/FB_Player_Run.FB_Player_Run")
      (else
        (Sprite|SetFlipbook (Variables|Default|GetSprite) "/Game/Animations/Character/Walk/FB_Player_Walk.FB_Player_Walk")))
    (else
      (Sprite|SetFlipbook (Variables|Default|GetSprite) "/Game/Animations/Character/Idle/FB_Player_Idle.FB_Player_Idle"))))

(fn UpdateRotation
  (Math|Float|CompareFloat (.x (Variables|/Script/Engine.MovementComponent|GetVelocity (Variables|Character|GetCharacterMovement))) 0.0
    (:>
      ;[1 1 1] Look right
      (bind _asplayer_controller (Utilities|Casting|CastToPlayerController (Pawn|GetController)))
      (Pawn|SetControlRotation _asplayer_controller (Math|Rotator|MakeRotator 0.0 0.0 0.0)))
    (:<
      ;[1 1 1] Look left
      (bind _asplayer_controller_2 (Utilities|Casting|CastToPlayerController (Pawn|GetController)))
      (Pawn|SetControlRotation _asplayer_controller_2 (Math|Rotator|MakeRotator 0.0 0.0 1.8e+02)))))