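; Side-scroller checkpoint that becomes the active checkpoint when the hero first enters its trigger, and lights up as a lantern.
; On BeginPlay it caches GM_SideScroller and creates a dynamic M_Custom_Lit material for its sprite.
; A one-shot trigger overlap registers the checkpoint with the game mode, then calls TriggerFlash, which sets the material's flash multiplier and color to light the lantern.
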(event OnComponentBeginOverlap(Trigget)
  (params (OverlappedComponent :type Primitive%20Component%20Object%20Reference) (OtherActor :type Actor%20Object%20Reference) (OtherComp :type Primitive%20Component%20Object%20Reference) (OtherBodyIndex :type Integer) (bFromSweep :type Boolean) (SweepResult :type Hit%20Result%20Structure%20%28by%20ref%29))
  (Utilities|Casting|CastToBP_Hero OtherActor)
  (Utilities|FlowControl|DoOnce false
    (:Completed
      (Variables|/Game/Blueprints/GM_SideScroller.GM_SideScroller_C|SetActiveCheckpoint (Variables|Default|GetGM%20Side%20Scroller) self)
      (CallFunction|TriggerFlash 2.0 "(R=1.000000,G=1.000000,B=1.000000,A=1.000000)"))))

(event Custom|TriggerFlash
  (params (FlashMultiplier :type Float%20%28single-precision%29) (FlashColor :type Linear%20Color%20Structure))
  ;[1 1 1] Trigger Flash when overlap to light the lantern
  (Rendering|Material|SetScalarParameterValue (Variables|Default|GetDynamicSpriteMaterial) "FlashMultiplier" FlashMultiplier :!class /Script/Engine.MaterialInstanceDynamic)
  (Rendering|Material|SetVectorParameterValue (Variables|Default|GetDynamicSpriteMaterial) "FlashColor" FlashColor :!class /Script/Engine.MaterialInstanceDynamic))

(event EventBeginPlay
  (bind _asgm_side_scroller (Utilities|Casting|CastToGM_SideScroller (Game|GetGameMode)))
  (Variables|Default|SetGM%20Side%20Scroller _asgm_side_scroller)
  (bind _returnvalue (Rendering|Material|CreateDynamicMaterialInstance (Variables|Default|Getcheckpoint) 0 "/Game/Assets/Materials/M_Custom_Lit.M_Custom_Lit" "None" :!class /Script/Engine.PrimitiveComponent))
  (Variables|Default|SetDynamicSpriteMaterial _returnvalue))

(event Collision|EventActorBeginOverlap
  (params (OtherActor :type Actor%20Object%20Reference)))

(event EventTick
  (params (DeltaSeconds :type Float%20%28single-precision%29)))

(fn ConstructionScript)