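; BP_Ladder is a ladder actor that lets the player start climbing by switching the character to Flying movement.
; Overlapping LadderVolume sets an IsLadder flag, enables input and toggles the Usage component's visibility; leaving clears the flag and toggles it again.
; An input action checks that flag and whether E is held before setting Flying mode.
; Leaving the volume keeps input enabled, and nothing here restores the previous movement mode.
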(event OnComponentBeginOverlap(LadderVolume)
  (params (OverlappedComponent :type Primitive%20Component%20Object%20Reference) (OtherActor :type Actor%20Object%20Reference) (OtherComp :type Primitive%20Component%20Object%20Reference) (OtherBodyIndex :type Integer) (bFromSweep :type Boolean) (SweepResult :type Hit%20Result%20Structure%20%28by%20ref%29))
  (Input|EnableInput (Game|GetPlayerController 0))
  (Variables|Default|SetIsLadder true)
  (Rendering|ToggleVisibility (Variables|Default|GetUsage) false))

(event OnComponentEndOverlap(LadderVolume)
  (params (OverlappedComponent :type Primitive%20Component%20Object%20Reference) (OtherActor :type Actor%20Object%20Reference) (OtherComp :type Primitive%20Component%20Object%20Reference) (OtherBodyIndex :type Integer))
  (Input|EnableInput (Game|GetPlayerController 0))
  (Variables|Default|SetIsLadder false)
  (Rendering|ToggleVisibility (Variables|Default|GetUsage) false))

(event Input|EnhancedActionEvents|EnhancedInputAction
  (params (ActionValue :type Boolean) (ElapsedSeconds :type Float%20%28double-precision%29) (TriggeredSeconds :type Float%20%28double-precision%29) (InputAction :type Input%20Action%20Object%20Reference :default "IA_Climb"))
  (if (Variables|Default|GetIsLadder)
    (if (Game|Player|IsInputKeyDown (Game|GetPlayerController 0) "E")
      (Pawn|Components|CharacterMovement|SetMovementMode (Variables|/Script/Engine.Character|GetCharacterMovement (Game|GetPlayerCharacter 0)) "MOVE_Flying" 0))))

(fn ConstructionScript)