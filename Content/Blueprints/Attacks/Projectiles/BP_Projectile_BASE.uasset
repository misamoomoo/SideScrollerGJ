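; Base projectile actor for attacks, carrying a faction and a damage value.
; Overlapping a BP_Character_BASE of a different faction applies damage to it, while same-faction characters and non-character overlaps are ignored.
; Both a damaging overlap and any blocking hit on the sphere call BlamEffect, which spawns the BP_VFX_ShotHit effect at the projectile's transform and destroys it.
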(event OnComponentHit(Sphere)
  (params (HitComponent :type Primitive%20Component%20Object%20Reference) (OtherActor :type Actor%20Object%20Reference) (OtherComp :type Primitive%20Component%20Object%20Reference) (NormalImpulse :type Vector :default "0, 0, 0") (Hit :type Hit%20Result%20Structure%20%28by%20ref%29))
  (CallFunction|BlamEffect))

(event OnComponentBeginOverlap(Sphere)
  (params (OverlappedComponent :type Primitive%20Component%20Object%20Reference) (OtherActor :type Actor%20Object%20Reference) (OtherComp :type Primitive%20Component%20Object%20Reference) (OtherBodyIndex :type Integer) (bFromSweep :type Boolean) (SweepResult :type Hit%20Result%20Structure%20%28by%20ref%29))
  ;[1 1 1] Destroy actor if not the same faction
  (bind _asbp_character_base (Utilities|Casting|CastToBP_Character_BASE OtherActor))
  (if (Utilities|Enum|NotEqual(Enum) (Variables|/Game/Blueprints/Characters/BP_Character_BASE.BP_Character_BASE_C|GetFaction _asbp_character_base) (Variables|Default|GetFaction))
    (Game|Damage|ApplyDamage _asbp_character_base (Variables|Default|GetProjectileDamage) 0 self)
    (CallFunction|BlamEffect)))

(event EventTick
  (params (DeltaSeconds :type Float%20%28single-precision%29)))

(event EventBeginPlay)

(fn ConstructionScript)

(fn PlayHitEffects
  (Game|SpawnActorfromClass "/Game/Blueprints/Attacks/VFX/BP_VFX_ShotHit.BP_VFX_ShotHit_C" (Math|Transform|MakeTransform (Transformation|GetActorLocation) (Transformation|GetActorRotation) "1.000000,1.000000,1.000000") "AlwaysSpawn" "MultiplyWithRoot" 0 0))

(fn BlamEffect
  (CallFunction|PlayHitEffects)
  (Actor|DestroyActor))