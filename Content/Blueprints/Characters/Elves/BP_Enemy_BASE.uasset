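; BP_Enemy_BASE is a base Blueprint for enemy characters that removes the enemy once it is defeated.
; On BeginPlay it binds OnDefeated to the Defeated event, and that handler destroys the actor.
; The Destroyed event spawns a BP_VFX_EnemyBlam effect at the actor's location and rotation, so the effect follows any destruction, not only defeat.
; Tick and the construction script only call their parent versions.
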(event Custom|OnDefeated
  (Actor|DestroyActor))

(event EventBeginPlay
  (|CallParentFunction)
  (EventDispatchers|BindEventtoDefeated (delegate Custom|OnDefeated)))

(event EventTick
  (params (DeltaSeconds :type Float%20%28single-precision%29))
  (|CallParentFunction DeltaSeconds))

(event EventDestroyed
  (Game|SpawnActorfromClass "/Game/Blueprints/Attacks/VFX/BP_VFX_EnemyBlam.BP_VFX_EnemyBlam_C" (Math|Transform|MakeTransform (Transformation|GetActorLocation) (Transformation|GetActorRotation) "1.000000,1.000000,1.000000") "AlwaysSpawn" "MultiplyWithRoot" 0 0))

(fn ConstructionScript
  (|CallParentFunction))