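; BP_Enemy_Elf_Small is a Paper2D small elf enemy that walks along its facing direction and calls TurnCharacter when its wall detector begins an overlap or its ledge detector ends one.
; Each tick, UpdateAnim switches the body flipbook and dress sprite between walk and idle based on velocity.
; Tick also repositions the separate Dress sprite slightly behind and above the actor at a fixed Y depth to layer the outfit.
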(event OnComponentBeginOverlap(WallDetector)
  (params (OverlappedComponent :type Primitive%20Component%20Object%20Reference) (OtherActor :type Actor%20Object%20Reference) (OtherComp :type Primitive%20Component%20Object%20Reference) (OtherBodyIndex :type Integer) (bFromSweep :type Boolean) (SweepResult :type Hit%20Result%20Structure%20%28by%20ref%29))
  (CallFunction|TurnCharacter))

(event OnComponentEndOverlap(LedgeDetector)
  (params (OverlappedComponent :type Primitive%20Component%20Object%20Reference) (OtherActor :type Actor%20Object%20Reference) (OtherComp :type Primitive%20Component%20Object%20Reference) (OtherBodyIndex :type Integer))
  (CallFunction|TurnCharacter))

(event Custom|WalkForward
  (params (ScaleValue :type Float%20%28single-precision%29))
  (Pawn|Input|AddMovementInput (Transformation|GetActorForwardVector) ScaleValue false))

(event EventBeginPlay
  (|CallParentFunction))

(event Collision|EventActorBeginOverlap
  (params (OtherActor :type Actor%20Object%20Reference))
  (|CallParentFunction OtherActor) ; This node is disabled and will not be called.\nDrag off pins to build functionality.
)

(event EventTick
  (params (DeltaSeconds :type Float%20%28single-precision%29))
  (bind _returnvalue (Transformation|GetActorLocation))
  (|CallParentFunction DeltaSeconds)
  (CallFunction|UpdateAnim)
  (Transformation|SetWorldLocation (Variables|Default|Getdress) (Math|Vector|MakeVector (+ (.x _returnvalue) (* (.x (Transformation|GetActorForwardVector)) -2.5)) 0.1 (+ (.z _returnvalue) 4.0)) false false))

(fn ConstructionScript
  (|CallParentFunction))

(fn UpdateAnim
  (if (!= (Math|Vector|VectorLength (Transformation|GetVelocity)) 0.0)
    (Rendering|Components|Sprite|SetSprite (Variables|Default|Getdress) "/Game/Assets/Sprites/elves/Female_outfit_1_3_4_Sprite.Female_outfit_1_3_4_Sprite")
    (Sprite|SetFlipbook (Variables|Default|GetSprite) "/Game/Assets/Animations/elves/FB_Elf_Walk.FB_Elf_Walk")
    (else
      (Rendering|Components|Sprite|SetSprite (Variables|Default|Getdress) "/Game/Assets/Sprites/elves/Female_outfit_1_Sprite.Female_outfit_1_Sprite")
      (Sprite|SetFlipbook (Variables|Default|GetSprite) "/Game/Assets/Animations/elves/FB_Elf_Idle.FB_Elf_Idle"))))