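; Side-scroller player hero Blueprint handling Enhanced Input movement along X, jumping, and energy-limited projectile shooting.
; Overlapping an enemy capsule applies damage, and surviving a hit triggers temporary invincibility with timer-driven sprite flicker and ignored Pawn collision.
; Defeat runs a respawn sequence that disables collision, detaches the camera arm, fades out, asks GM_SideScroller to respawn the player, fades in and destroys this actor.
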(event OnComponentBeginOverlap(CapsuleComponent)
  (params (OverlappedComponent :type Primitive%20Component%20Object%20Reference) (OtherActor :type Actor%20Object%20Reference) (OtherComp :type Primitive%20Component%20Object%20Reference) (OtherBodyIndex :type Integer) (bFromSweep :type Boolean) (SweepResult :type Hit%20Result%20Structure%20%28by%20ref%29))
  ;[1 1 1] Getting Hit
  (bind _asbp_enemy_base (Utilities|Casting|CastToBP_Enemy_BASE OtherActor))
  (if (== (Variables|/Script/Engine.Character|GetCapsuleComponent _asbp_enemy_base) OtherComp)
    (Game|Damage|ApplyDamage self (Variables|Default|GetOverlapDamage) 0 0)))

(event Custom|TriggerInvincibility
  ;[1 1 1] Become Invincible for a bit after being hit and then reset
  (Collision|SetCollisionResponsetoChannel (Variables|Default|GetCapsuleComponent) "ECC_Pawn" "ECR_Ignore")
  (bind _returnvalue (Utilities|Time|SetTimerbyEvent (EventDispatchers|CreateEvent :!event ToggleSpriteFlicker) (Variables|Default|GetSpriteFlickerInterval) true))
  (Variables|Default|SetFlickerHandle _returnvalue)
  (Utilities|FlowControl|RetriggerableDelay (Variables|Default|GetInvincibilityDuration))
  ;;[1 1 1] Stop flickering and reset visibility just in case it disappears
  (Utilities|Time|ClearandInvalidateTimerbyHandle (Variables|Default|GetFlickerHandle))
  (Collision|SetCollisionResponsetoChannel (Variables|Default|GetCapsuleComponent) "ECC_Pawn" "ECR_Overlap")
  (Rendering|SetVisibility (Variables|Default|GetSprite) true true))

(event Custom|OnDefeated
  ;[1 1 1] Add action mapping, respawning
  (|RespawnSequence))

(event Input|EnhancedActionEvents|EnhancedInputActionIA_Move
  (params (ActionValue :type Vector%202D%20Structure) (ElapsedSeconds :type Float%20%28double-precision%29) (TriggeredSeconds :type Float%20%28double-precision%29) (InputAction :type Input%20Action%20Object%20Reference :default "/Game/Input/Actions/IA_Move.IA_Move"))
  ;[1 1 1] Basic Movement
  (if (Variables|Default|GetIsBeingControlled)
    (Utilities|FlowControl|Sequence
      (:then_0
        (CallFunction|UpdateRotation (.x ActionValue))
        (Pawn|Input|AddMovementInput "1.000000,0.000000,0.000000" (.x ActionValue) false)))))

(event Input|EnhancedActionEvents|EnhancedInputActionIA_Jump
  (params (ActionValue :type Boolean) (ElapsedSeconds :type Float%20%28double-precision%29) (TriggeredSeconds :type Float%20%28double-precision%29) (InputAction :type Input%20Action%20Object%20Reference :default "/Game/Input/Actions/IA_Jump.IA_Jump"))
  ;[1 1 1] Jumping
  (:Started
    (if (Variables|Default|GetIsBeingControlled)
      (Character|Jump)))
  (:Canceled
    (Character|StopJumping :!label _label))
  (:Completed
    (goto _label)))

(event Input|EnhancedActionEvents|EnhancedInputActionIA_Shoot
  (params (ActionValue :type Boolean) (ElapsedSeconds :type Float%20%28double-precision%29) (TriggeredSeconds :type Float%20%28double-precision%29) (InputAction :type Input%20Action%20Object%20Reference :default "/Game/Input/Actions/IA_Shoot.IA_Shoot"))
  (bind _self self)
  (bind _shootpos (Variables|Default|GetShootPos))
  ;[1 1 1] Shooting Ability
  (:Started
    (if (and (Variables|Default|GetIsBeingControlled) (> (Variables|Default|GetShotEnergy) 0))
      (Math|Integer|DecrementInt (Variables|Default|GetShotEnergy)
        (:%20%20
          (Variables|Default|SetIsShooting true)
          (Game|SpawnActorfromClass "/Game/Blueprints/Attacks/Projectiles/Hero/BP_PlayerProjectile_Regular.BP_PlayerProjectile_Regular_C" (Math|Transform|MakeTransform (Transformation|GetWorldLocation _shootpos) (Transformation|GetWorldRotation _shootpos) "1.000000,1.000000,1.000000") "AlwaysSpawn" "MultiplyWithRoot" _self _self)
          (Utilities|FlowControl|RetriggerableDelay (Variables|Default|GetShootDuration))
          (Variables|Default|SetIsShooting false))))))

(event EventBeginPlay
  ;[1 1 1] Add action mapping, respawning
  (|CallParentFunction)
  (Utilities|FlowControl|Sequence
    (:then_0
      (bind _asgm_side_scroller (Utilities|Casting|CastToGM_SideScroller (Game|GetGameMode)))
      (Variables|Default|SetGM%20Side%20Scroller _asgm_side_scroller)
      (bind _asplayer_controller (Utilities|Casting|CastToPlayerController (Pawn|GetController)))
      (Input|AddMappingContext (PlayerController|LocalPlayerSubsystems|GetEnhancedInputLocalPlayerSubsystem _asplayer_controller) "/Game/Input/IMC_SideScroller.IMC_SideScroller" 0 "(bIgnoreAllPressedKeysUntilRelease=True,bForceImmediately=False,bNotifyUserSettings=False)"))
    (:then_1
      (Variables|Default|SetBase%20Lateral%20Friction (Variables|/Script/Engine.CharacterMovementComponent|GetFallingLateralFriction (Variables|Character|GetCharacterMovement))))
    (:then_2
      (EventDispatchers|BindEventtoDefeated (delegate Custom|OnDefeated)))))

(event Game|Damage|EventAnyDamage
  (params (Damage :type Float%20%28single-precision%29) (DamageType :type Damage%20Type%20Object%20Reference) (InstigatedBy :type Controller%20Object%20Reference) (DamageCauser :type Actor%20Object%20Reference))
  ;[1 1 1] Become Invincible for a bit after being hit and then reset
  (|CallParentFunction Damage DamageType InstigatedBy DamageCauser)
  (if (not (Variables|/Game/Blueprints/Components/BPC_Vitality.BPC_Vitality_C|GetIsDefeated (Variables|Default|GetBPC_Vitality)))
    (CallFunction|TriggerInvincibility)))

(event Input|KeyboardEvents|Q
  (params (Key :type Key%20Structure :default "None"))
  ;[1 1 1] Dirty quit
  (:Pressed
    (Game|QuitGame 0 "Quit" false)))

(fn ConstructionScript
  (|CallParentFunction))

(fn UpdateRotation
  (params (Direction :type Float%20%28double-precision%29))
  (Pawn|SetControlRotation (Pawn|GetController) (Math|Rotator|SelectRotator (Math|Rotator|MakeRotator 0.0 0.0 0.0) (Math|Rotator|MakeRotator 0.0 0.0 1.8e+02) (!= Direction 0.0))))

(fn RestoreShots
  (Math|Integer|IncrementInt (Variables|Default|GetShotEnergy)))

(fn ToggleSpriteFlicker
  (bind _sprite (Variables|Default|GetSprite))
  (Rendering|SetVisibility _sprite (not (Variables|/Script/Engine.SceneComponent|GetbVisible _sprite)) true))