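; BP_Character_BASE is a base character Blueprint that handles taking damage and a hit-flash effect on its sprite.
; Damage goes to the BPCVitality component, then either calls Defeated when the character is defeated or triggers a flash, and is ignored once already defeated.
; The flash sets color and intensity on a dynamic lit sprite material created at BeginPlay, then a timeline fades the intensity to zero at an adjustable play rate.
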(event Custom|TriggerFlash
  (params (FlashMultiplier :type Float%20%28single-precision%29) (FlashColor :type Linear%20Color%20Structure))
  ;[1 1 1] Trigger Flash when hit then return to normal
  (Rendering|Material|SetScalarParameterValue (Variables|Default|GetDynamicSpriteMaterial) "FlashMultiplier" FlashMultiplier :!class /Script/Engine.MaterialInstanceDynamic)
  (Rendering|Material|SetVectorParameterValue (Variables|Default|GetDynamicSpriteMaterial) "FlashColor" FlashColor :!class /Script/Engine.MaterialInstanceDynamic)
  (Components|Timeline|SetPlayRate (Variables|Default|GetFadeSpriteFlash) (Variables|Default|GetSpriteFlashPlayRate))
  (bind _alpha (Timeline|FadeSpriteFlash PlayFromStart)
    (:Update
      (Rendering|Material|SetScalarParameterValue (Variables|Default|GetDynamicSpriteMaterial) "FlashMultiplier" (Math|Float|Lerp FlashMultiplier 0.0 _alpha) :!class /Script/Engine.MaterialInstanceDynamic))))

(event EventBeginPlay
  (bind _returnvalue (Rendering|Material|CreateDynamicMaterialInstance (Variables|Default|GetSprite) 0 "/Game/Assets/Materials/M_Custom_Lit.M_Custom_Lit" "None" :!class /Script/Engine.PrimitiveComponent))
  (Variables|Default|SetDynamicSpriteMaterial _returnvalue))

(event Collision|EventActorBeginOverlap
  (params (OtherActor :type Actor%20Object%20Reference)))

(event EventTick
  (params (DeltaSeconds :type Float%20%28single-precision%29)))

(event Game|Damage|EventAnyDamage
  (params (Damage :type Float%20%28single-precision%29) (DamageType :type Damage%20Type%20Object%20Reference) (InstigatedBy :type Controller%20Object%20Reference) (DamageCauser :type Actor%20Object%20Reference))
  ;[1 1 1] Reduce health from damage then destroy if defeated
  (if (not (Variables|/Game/Blueprints/Components/BPC_Vitality.BPC_Vitality_C|GetIsDefeated (Variables|Default|GetBPC_Vitality)))
    (Default|ReceiveDamage (Variables|Default|GetBPC_Vitality) Damage)
    (if (Variables|/Game/Blueprints/Components/BPC_Vitality.BPC_Vitality_C|GetIsDefeated (Variables|Default|GetBPC_Vitality))
      (Default|CallDefeated)
      (else
        (CallFunction|TriggerFlash 1e+01 "(R=0.348958,G=0.534112,B=1.000000,A=1.000000)")))))

(fn ConstructionScript)