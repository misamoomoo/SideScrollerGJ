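; BP_Hero is the player character for a side-scroller, with running, jumping and ladder climbing through Enhanced Input.
; BeginPlay adds the mapping context; horizontal input moves along X and snaps control yaw to flip facing.
; Vertical input moves along Z on an overlapping ladder; the first upward push sets IsClimbing, which blocks horizontal movement, switches to Flying and jumps the animation to climbing.
; A debug-style Q key quits the game.
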(event Input|EnhancedActionEvents|EnhancedInputActionIA_Jump
  (params (ActionValue :type Boolean) (ElapsedSeconds :type Float%20%28double-precision%29) (TriggeredSeconds :type Float%20%28double-precision%29) (InputAction :type Input%20Action%20Object%20Reference :default "/Game/Input/Actions/IA_Jump.IA_Jump"))
  ;[1 1 1] Jump movement
  (:Started
    (Character|Jump))
  (:Canceled
    (Character|StopJumping :!label _label))
  (:Completed
    (goto _label)))

(event Input|EnhancedActionEvents|EnhancedInputActionIA_Move
  (params (ActionValue :type Vector%202D%20Structure) (ElapsedSeconds :type Float%20%28double-precision%29) (TriggeredSeconds :type Float%20%28double-precision%29) (InputAction :type Input%20Action%20Object%20Reference :default "/Game/Input/Actions/IA_Move.IA_Move"))
  ;[1 1 1] Basic movement
  (:Triggered
    (Utilities|FlowControl|Sequence
      (:then_0
        (if (not (Variables|Default|GetIsClimbing))
          (Pawn|Input|AddMovementInput "1.000000,0.000000,0.000000" (.x ActionValue) false)
          ;;[1 1 1] flip character if moving left
          (CallFunction|UpdateRotation (.x ActionValue))))
      (:then_1
        ;;[1 1 1] Climb Ladder
        (CallFunction|ClimbLadder (.y ActionValue))))))

(event EventBeginPlay
  ;[1 1 1] Add input map
  (bind _asplayer_controller (Utilities|Casting|CastToPlayerController (Pawn|GetController)))
  (Input|AddMappingContext (PlayerController|LocalPlayerSubsystems|GetEnhancedInputLocalPlayerSubsystem _asplayer_controller) "/Game/Input/IMC_SideScroller.IMC_SideScroller" 0 "(bIgnoreAllPressedKeysUntilRelease=True,bForceImmediately=False,bNotifyUserSettings=False)"))

(event Input|KeyboardEvents|Q
  (params (Key :type Key%20Structure :default "None"))
  ;[1 1 1] Dirty quit
  (:Pressed
    (Game|QuitGame 0 "Quit" false)))

(fn ConstructionScript
  (|CallParentFunction))

(fn UpdateRotation
  (params (Direction :type Float%20%28double-precision%29))
  (Pawn|SetControlRotation (Pawn|GetController) (Math|Rotator|SelectRotator (Math|Rotator|MakeRotator 0.0 0.0 0.0) (Math|Rotator|MakeRotator 0.0 0.0 1.8e+02) (>= Direction 0.0))))

(fn ClimbLadder
  (params (Direction :type Float%20%28double-precision%29))
  (bind _charactermovement (Variables|Character|GetCharacterMovement))
  (Variables|Default|GetOverlappingLadder
    (:then
      (Pawn|Input|AddMovementInput "0.000000,0.000000,1.000000" Direction false)
      (if (> Direction 0.0)
        (Utilities|FlowControl|DoOnce false
          (:Completed
            (Variables|Default|SetIsClimbing true)
            (Class|PaperZDAnimInstance|JumptoNode (Variables|/Script/PaperZD.PaperZDAnimationComponent|GetAnimInstance (Variables|Default|GetAnimationComponent)) "JumpClimb" "None")
            (Variables|/Script/Engine.MovementComponent|SetVelocity _charactermovement "0, 0, 0")
            (Pawn|Components|CharacterMovement|SetMovementMode _charactermovement "MOVE_Flying" 0)))))
    (:else)))